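; BP_PlayerCharacter is the networked shooter player character, with separate first-person and third-person guns.
; BeginPlay registers the third-person mesh and death camera, and Tick calls the server-driven rotation update.
; A delayed custom event sets gun visibility, showing the shadowless first-person gun only to the owner and hiding the third-person gun from them, then refreshes the HUD.
; Shoot and reload inputs go to the first-person child weapon actor.
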(event Input|EnhancedActionEvents|EnhancedInputActionIA_Shoot
  (params (ActionValue :type Boolean) (ElapsedSeconds :type Float%20%28double-precision%29) (TriggeredSeconds :type Float%20%28double-precision%29) (InputAction :type Input%20Action%20Object%20Reference :default "/Game/FirstPerson/Input/Actions/IA_Shoot.IA_Shoot"))
  (bind _asweapon_actor (Utilities|Casting|CastToWeaponActor (Variables|/Script/Engine.ChildActorComponent|GetChildActor (Variables|Default|GetFP_Gun))))
  (Class|WeaponActor|PrimaryFire _asweapon_actor true))

(event Input|EnhancedActionEvents|EnhancedInputActionIA_Reload
  (params (ActionValue :type Boolean) (ElapsedSeconds :type Float%20%28double-precision%29) (TriggeredSeconds :type Float%20%28double-precision%29) (InputAction :type Input%20Action%20Object%20Reference :default "/Game/_Game/CustomInput/IA_Reload.IA_Reload"))
  (bind _asweapon_actor (Utilities|Casting|CastToWeaponActor (Variables|/Script/Engine.ChildActorComponent|GetChildActor (Variables|Default|GetFP_Gun))))
  (Class|WeaponActor|Reload _asweapon_actor))

(event EventBeginPlay
  (Class|MyFTCharacter|SetThirdPersonMesh (Variables|Default|GetServe_TP_Mesh))
  (Variables|Default|SetTPDeath_Camera self (Variables|Default|GetDeathCamera)))

(event Collision|EventActorBeginOverlap
  (params (OtherActor :type Actor%20Object%20Reference)))

(event EventTick
  (params (DeltaSeconds :type Float%20%28single-precision%29))
  (Class|MyFTCharacter|FromServerSetCharacterRotation))

(event EventOnCustomEvent
  (Utilities|FlowControl|Delay 1.0)
  (CallFunction|ConfigureWeaponAppearence)
  (Utilities|FlowControl|Delay 1.0)
  (Class|MyFTCharacter|RefreshHUD))

(fn ConstructionScript)

(fn ConfigureWeaponAppearence
  (Utilities|FlowControl|Sequence
    (:then_0
      (bind _asbp_gun (Utilities|Casting|CastToBP_Gun (Variables|/Script/Engine.ChildActorComponent|GetChildActor (Variables|Default|GetFP_Gun)))
        (:then
          (Rendering|SetOnlyOwnerSee (Variables|/Script/FireTeam.WeaponActor|GetWeaponMesh _asbp_gun) true :!class /Script/Engine.PrimitiveComponent)
          (Rendering|SetCastShadow (Variables|/Script/FireTeam.WeaponActor|GetWeaponMesh _asbp_gun) false))
        (:CastFailed
          (Development|PrintString "FP_Gun childactor component cast to BP_Gun class failed" true true "(R=0.000000,G=0.660000,B=1.000000,A=1.000000)" 1e+02))))
    (:then_1
      (bind _asbp_gun_2 (Utilities|Casting|CastToBP_Gun (Variables|/Script/Engine.ChildActorComponent|GetChildActor (Variables|Default|GetServe_TP_Gun)))
        (:then
          (Class|PrimitiveComponent|SetOwnerNoSee (Variables|/Script/FireTeam.WeaponActor|GetWeaponMesh _asbp_gun_2) true))
        (:CastFailed
          (Development|PrintString "Serve_TP_Gun childactor component cast to BP_Gun class failed" true true "(R=0.000000,G=0.660000,B=1.000000,A=1.000000)" 1e+02))))))