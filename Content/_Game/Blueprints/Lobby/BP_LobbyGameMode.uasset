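; Lobby game mode that tracks joining players and keeps each player controller's player list up to date.
; On PostLogin it stores each BP_LobbyPlayerController and builds its PlayerInfo from the PlayerState name, with default level and not-ready state.
; It then passes the full info array to every connected controller through UpdatePlayerList.
; Only logins update the list; the file has no logout handling.
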(event EventBeginPlay)

(event EventTick
  (params (DeltaSeconds :type Float%20%28single-precision%29)))

(event EventPostLogin
  (params (NewPlayer :type Player%20Controller%20Object%20Reference))
  (bind _asbp_lobby_player_controller (Utilities|Casting|CastToBP_LobbyPlayerController NewPlayer))
  (Utilities|Array|Add (Variables|Default|GetConnectedPlayers) _asbp_lobby_player_controller)
  (bind _output_get (Variables|/Game/_Game/Blueprints/Lobby/BP_LobbyPlayerController.BP_LobbyPlayerController_C|SetPlayerInfo _asbp_lobby_player_controller (Utilities|Struct|MakeF_PlayerInfo (PlayerState|GetPlayerName (Variables|/Script/Engine.Controller|GetPlayerState NewPlayer)) 0 false)))
  (Utilities|Array|Add (Variables|Default|GetConnectedPlayersInfo) _output_get)
  (for _array_element (Variables|Default|GetConnectedPlayers)
    (Default|UpdatePlayerList _array_element (Variables|Default|GetConnectedPlayersInfo))))

(fn ConstructionScript)